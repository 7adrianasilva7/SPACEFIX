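; BP_Rail is a satellite rail that tracks its own health and can be damaged and repaired.
; DamageRail flags the rail as damaged and removes a fixed chunk of RailHP, while RepairRail adds RepairAmount, both clamped between zero and full.
; The damaged flag clears only when repairs restore RailHP to full.
; The construction script is empty, and nothing in the file calls either function.
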(fn `DamageRail`
  (set `self.IsRailDamaged` true)
  (set `self.RailHP` (`KismetMathLibrary.FClamp` (- (`self.RailHP`) 50.0) 0.0 100.0)))

(fn `RepairRail`
  (bind _output_get (set `self.RailHP` (`KismetMathLibrary.FClamp` (+ (`self.RepairAmount`) (`self.RailHP`)) 0.0 100.0)))
  (if (>= _output_get 100.0)
    (set `self.IsRailDamaged` false)))

(fn `UserConstructionScript`)