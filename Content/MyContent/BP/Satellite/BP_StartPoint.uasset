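; BP_StartPoint is a satellite deposit point where the player returns a carried satellite.
; Any DepositZone overlap checks player 0, moves its carried satellite to that satellite's StartLocation and clears the carried reference.
; The satellite's rail and pickup flags and the player's carrying flag take the SetActorLocation result.
; ShowDepositEffect starts a Niagara effect and beep; depositing calls HideDepositEffect on the first BP_StartPoint found, not necessarily itself.
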(event `self.ReceiveBeginPlay`
  (bind _linkedsatellite (`self.LinkedSatellite`))
  (`/Engine/EditorBlueprintResources/StandardMacros.IsValid` _linkedsatellite
    (:`Is Valid`
      (set `self.LinkedSatellite` _linkedsatellite))))

(event `self.DepositZone.OnComponentBeginOverlap`
  (params (OverlappedComponent :type "PrimitiveComponent Object Reference") (OtherActor :type "Actor Object Reference") (OtherComp :type "PrimitiveComponent Object Reference") (OtherBodyIndex :type Integer) (bFromSweep :type Boolean) (SweepResult :type "HitResult Structure (by ref)"))
  (bind _bp_firstpersonref (`self.BP_FirstPersonRef`))
  (bind _asbp_first_person_character (cast `/Game/FirstPerson/Blueprints/BP_FirstPersonCharacter` (`GameplayStatics.GetPlayerCharacter` 0)))
  (bind _output_get (set `self.BP_FirstPersonRef` _asbp_first_person_character))
  (if (`/Game/FirstPerson/Blueprints/BP_FirstPersonCharacter.IsCarryingSatellite` _output_get)
    (bind _carriedsatellite (`/Game/FirstPerson/Blueprints/BP_FirstPersonCharacter.CarriedSatellite` _asbp_first_person_character))
    (`/Engine/EditorBlueprintResources/StandardMacros.IsValid` _carriedsatellite
      (:`Is Valid`
        (set `/Game/MyContent/BP/Satellite/BP_Satellite.IsCarriedByPlayer` false _carriedsatellite)
        (bind (_sweephitresult _returnvalue) (`self.K2_SetActorLocation` _carriedsatellite (`/Game/MyContent/BP/Satellite/BP_Satellite.StartLocation` _carriedsatellite) false false))
        (set `/Game/MyContent/BP/Satellite/BP_Satellite.IsOnRail` _returnvalue _carriedsatellite)
        (set `/Game/MyContent/BP/Satellite/BP_Satellite.IsPickupable` _returnvalue _carriedsatellite)
        (set `/Game/FirstPerson/Blueprints/BP_FirstPersonCharacter.IsCarryingSatellite` _returnvalue _bp_firstpersonref)
        (set `/Game/FirstPerson/Blueprints/BP_FirstPersonCharacter.CarriedSatellite` null _bp_firstpersonref)
        (bind _outactors (`GameplayStatics.GetAllActorsOfClass` "BP_StartPoint_C"))
        (`self.HideDepositEffect` (`|GetArrayItem` _outactors))))))

(event `ShowDepositEffect`
  (bind _returnvalue (`NiagaraFunctionLibrary.SpawnSystemAttached` "/Game/MyContent/NS/NS_DepositSat.NS_DepositSat" (`self.RootComponent`) "None" (`self.K2_GetActorLocation`) (struct) "KeepRelativeOffset"))
  (set `self.NiagaraComponent` _returnvalue)
  (bind _returnvalue_2 (`GameplayStatics.SpawnSoundAtLocation` "/Game/MyContent/SFX/beep.beep" (`self.K2_GetActorLocation`) (struct) 0.1 1.0 0.0 null null))
  (set `self.AudioComponent` _returnvalue_2))

(event `HideDepositEffect`
  (bind _niagaracomponent (`self.NiagaraComponent`))
  (bind _audiocomponent (`self.AudioComponent`))
  (`/Engine/EditorBlueprintResources/StandardMacros.IsValid` _niagaracomponent
    (:`Is Valid`
      (`ActorComponent.Deactivate` _niagaracomponent)
      (set `self.NiagaraComponent` null)
      (`/Engine/EditorBlueprintResources/StandardMacros.IsValid` _audiocomponent
        (:`Is Valid`
          (`AudioComponent.Stop` _audiocomponent)
          (set `self.AudioComponent` null))))))

(fn `UserConstructionScript`)