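; Wall lamp actor that signals satellite state, blinking red during an attack and flashing green on delivery.
; The construction script configures its dynamic and GI point lights and emissive material from variables.
; A looping timer from BeginPlay triggers a randomized visibility flicker.
; Red alert toggles color and material through a timer-driven FlipFlop until stopped; green reverts to white after a delay, though intensity stays boosted.
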(event `StartBlinkRed`
  ; Quand le satellite ce fait attaquer, les lumiere deviennent rouge
  (bind _returnvalue (`KismetSystemLibrary.K2_SetTimer` null "BlinkRed" 0.3 true))
  (set `self.BlinkTimerHandle` _returnvalue)
  (set `self.IsBlinkingRed` true))

(event `BlinkRed`
  (bind _sm_wall_lamp_a (`self.SM_Wall_lamp_A`))
  ; Quand le satellite ce fait attaquer, les lumiere deviennent rouge
  (`/Engine/EditorBlueprintResources/StandardMacros.FlipFlop`
    (:`A`
      (`PrimitiveComponent.SetMaterial` _sm_wall_lamp_a 1 "/Game/MyContent/Materials/M_LampRed.M_LampRed")
      (`LightComponent.SetLightColor` (`self.LIT_PointLight_DynamicShortRange_01A`) (struct :`R` 1.0 :`A` 1.0) true)
      (`LightComponent.SetLightColor` (`self.LIT_PointLight_GI_01A1`) (struct :`R` 1.0 :`A` 1.0) true)
      (`LightComponent.SetIntensity` (`self.LIT_PointLight_DynamicShortRange_01A`) 15000.0)
      (`LightComponent.SetIntensity` (`self.LIT_PointLight_GI_01A1`) 15000.0))
    (:`B`
      (`PrimitiveComponent.SetMaterial` _sm_wall_lamp_a 1 "/Game/Fab/sci-fi_Lamp/Material/M_Emissive.M_Emissive")
      (`LightComponent.SetLightColor` (`self.LIT_PointLight_DynamicShortRange_01A`) (struct :`R` 1.0 :`G` 1.0 :`B` 1.0 :`A` 1.0) true)
      (`LightComponent.SetLightColor` (`self.LIT_PointLight_GI_01A1`) (struct :`R` 1.0 :`G` 1.0 :`B` 1.0 :`A` 1.0) true))))

(event `StopBlinkRed`
  ; Quand le satellite ce fait attaquer, les lumiere deviennent rouge
  (`KismetSystemLibrary.K2_ClearAndInvalidateTimerHandle` (`self.BlinkTimerHandle`))
  (set `self.IsBlinkingRed` false)
  (`LightComponent.SetLightColor` (`self.LIT_PointLight_DynamicShortRange_01A`) (struct :`R` 1.0 :`G` 1.0 :`B` 1.0 :`A` 1.0) true)
  (`LightComponent.SetLightColor` (`self.LIT_PointLight_GI_01A1`) (struct :`R` 1.0 :`G` 1.0 :`B` 1.0 :`A` 1.0) true)
  (`PrimitiveComponent.SetMaterial` (`self.SM_Wall_lamp_A`) 1 "/Game/Fab/sci-fi_Lamp/Material/M_Emissive.M_Emissive")
  (`LightComponent.SetIntensity` (`self.LIT_PointLight_DynamicShortRange_01A`) 5000.0)
  (`LightComponent.SetIntensity` (`self.LIT_PointLight_GI_01A1`) 5000.0))

(event `BlinkGreen`
  (bind _lit_pointlight_dynamicshortrange_01a (`self.LIT_PointLight_DynamicShortRange_01A`))
  (bind _lit_pointlight_gi_01a1 (`self.LIT_PointLight_GI_01A1`))
  (bind _lit_pointlight_gi_01a1_2 (`self.LIT_PointLight_GI_01A1`))
  (bind _lit_pointlight_dynamicshortrange_01a_2 (`self.LIT_PointLight_DynamicShortRange_01A`))
  ; Quand le satellite est livré, les lumiere deviennent verte
  (`LightComponent.SetLightColor` _lit_pointlight_dynamicshortrange_01a (struct :`G` 1.0 :`A` 1.0) true)
  (`LightComponent.SetIntensity` _lit_pointlight_dynamicshortrange_01a 15000.0)
  (`LightComponent.SetLightColor` _lit_pointlight_gi_01a1 (struct :`G` 1.0 :`A` 1.0) true)
  (`LightComponent.SetIntensity` _lit_pointlight_gi_01a1 15000.0)
  (`PrimitiveComponent.SetMaterial` (`self.SM_Wall_lamp_A`) 1 "/Game/MyContent/Materials/M_LampGreen.M_LampGreen")
  (`KismetSystemLibrary.Delay` 1.0)
  (`LightComponent.SetLightColor` _lit_pointlight_dynamicshortrange_01a_2 (struct :`R` 1.0 :`G` 1.0 :`B` 1.0 :`A` 1.0) true)
  (`LightComponent.SetIntensity` _lit_pointlight_dynamicshortrange_01a_2 (`LightComponentBase.Intensity` _lit_pointlight_dynamicshortrange_01a_2))
  (`LightComponent.SetLightColor` _lit_pointlight_gi_01a1_2 (struct :`R` 1.0 :`G` 1.0 :`B` 1.0 :`A` 1.0) true)
  (`LightComponent.SetIntensity` _lit_pointlight_gi_01a1_2 (`LightComponentBase.Intensity` _lit_pointlight_gi_01a1_2))
  (`PrimitiveComponent.SetMaterial` (`self.SM_Wall_lamp_A`) 1 "/Game/Fab/sci-fi_Lamp/Material/MI_Emissive.MI_Emissive"))

(event `RandomFlick`
  ; Clignotement de lumiére
  (`SceneComponent.SetVisibility` (`self.LIT_PointLight_DynamicShortRange_01A`) false false)
  (`SceneComponent.SetVisibility` (`self.LIT_PointLight_GI_01A1`) false false)
  (`KismetSystemLibrary.Delay` (`KismetMathLibrary.RandomFloatInRange` 0.05 0.15))
  (`SceneComponent.SetVisibility` (`self.LIT_PointLight_DynamicShortRange_01A`) true false)
  (`SceneComponent.SetVisibility` (`self.LIT_PointLight_GI_01A1`) true false)
  (`KismetSystemLibrary.Delay` (`KismetMathLibrary.RandomFloatInRange` 0.05 0.1))
  (`SceneComponent.SetVisibility` (`self.LIT_PointLight_DynamicShortRange_01A`) false false)
  (`SceneComponent.SetVisibility` (`self.LIT_PointLight_GI_01A1`) false false)
  (`KismetSystemLibrary.Delay` 0.1)
  (`SceneComponent.SetVisibility` (`self.LIT_PointLight_DynamicShortRange_01A`) true false)
  (`SceneComponent.SetVisibility` (`self.LIT_PointLight_GI_01A1`) true false))

(event `self.ReceiveBeginPlay`
  ; Clignotement de lumiére
  (`KismetSystemLibrary.K2_SetTimerDelegate` (delegate `RandomFlick`) (`self.Time`) true))

(fn `UserConstructionScript`
  (bind _lit_pointlight_dynamicshortrange_01a (`self.LIT_PointLight_DynamicShortRange_01A`))
  (bind _lit_pointlight_gi_01a1 (`self.LIT_PointLight_GI_01A1`))
  (`|ExecutionSequence`
    (:`then_0`
      ;[1 1 1] Dynamic
      (`LightComponent.SetLightColor` _lit_pointlight_dynamicshortrange_01a (`self.Light Color`) true)
      (`LightComponent.SetIntensity` _lit_pointlight_dynamicshortrange_01a (`self.Intensity `))
      (`LocalLightComponent.SetAttenuationRadius` _lit_pointlight_dynamicshortrange_01a (`self.Radius `))
      (`PrimitiveComponent.SetMaterial` (`self.SM_Wall_lamp_A`) 1 (`self.Emissive Material`))
      (`LightComponent.SetVolumetricScatteringIntensity` _lit_pointlight_dynamicshortrange_01a (`self.Volumetric scattering Intensity `))
      (`LightComponent.SetIndirectLightingIntensity` _lit_pointlight_dynamicshortrange_01a (`self.Set Indirect Lighting Intensity`))
      (`LightComponentBase.SetCastShadows` _lit_pointlight_dynamicshortrange_01a (`self.Cast Shadow `))
      (`LightComponent.SetTemperature` _lit_pointlight_dynamicshortrange_01a (`self.Temperature`))
      (`PointLightComponent.SetSoftSourceRadius` _lit_pointlight_dynamicshortrange_01a (`self.Soft Source Radius`)))
    (:`then_1`
      ;[1 1 1] GI
      (`LightComponent.SetLightColor` _lit_pointlight_gi_01a1 (`self.Light Color`) true)
      (`LightComponent.SetIntensity` _lit_pointlight_gi_01a1 (`self.Intensity (GI)`))
      (`LocalLightComponent.SetAttenuationRadius` _lit_pointlight_gi_01a1 (`self.Radius (GI)`))
      (`LightComponentBase.SetCastShadows` _lit_pointlight_gi_01a1 (`self.Cast Shadow (GI)`))
      (`LightComponent.SetTemperature` _lit_pointlight_gi_01a1 (`self.Temperature`))
      (`LightComponent.SetIndirectLightingIntensity` _lit_pointlight_gi_01a1 (`self.Set Indirect Lighting Intensity (GI)`))
      (`PointLightComponent.SetSoftSourceRadius` _lit_pointlight_gi_01a1 (`self.Soft Source Radius (GI)`)))))