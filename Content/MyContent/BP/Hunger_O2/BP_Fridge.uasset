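; Fridge actor that opens its door for the first-person player and stocks food for them.
; Box overlap begin and end each play a sound and drive a separate timeline that rotates the door's yaw open or closed.
; On BeginPlay, SpawnFood spawns one BP_Food at the SpawnFood1 point and hands it a reference back to the fridge.
; StartCountdown is an empty event.
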(event `self.Box.OnComponentBeginOverlap`
  (params (OverlappedComponent :type "PrimitiveComponent Object Reference") (OtherActor :type "Actor Object Reference") (OtherComp :type "PrimitiveComponent Object Reference") (OtherBodyIndex :type Integer) (bFromSweep :type Boolean) (SweepResult :type "HitResult Structure (by ref)"))
  ; Ouvre/Ferme la porte du frigo
  (bind _asbp_first_person_character (cast `/Game/FirstPerson/Blueprints/BP_FirstPersonCharacter` OtherActor))
  (`GameplayStatics.PlaySound2D` "/Game/MyContent/SFX/openfridgedoor.openfridgedoor" 0.6 1.0 0.0 null _asbp_first_person_character)
  (bind (_direction _angle) (`Timeline|DoorTimeline` :!via `PlayFromStart`)
    (:`Update`
      (`SceneComponent.K2_SetRelativeRotation` (`self.fridgedoor`) (`KismetMathLibrary.MakeRotator` 0.0 0.0 _angle) false false))))

(event `self.Box.OnComponentEndOverlap`
  (params (OverlappedComponent :type "PrimitiveComponent Object Reference") (OtherActor :type "Actor Object Reference") (OtherComp :type "PrimitiveComponent Object Reference") (OtherBodyIndex :type Integer))
  ; Ouvre/Ferme la porte du frigo
  (bind _asbp_first_person_character (cast `/Game/FirstPerson/Blueprints/BP_FirstPersonCharacter` OtherActor))
  (`GameplayStatics.PlaySound2D` "/Game/MyContent/SFX/closefridgedoor.closefridgedoor" 0.6 1.0 0.0 null _asbp_first_person_character)
  (bind (_direction _angle) (`Timeline|Chronologie` :!via `ReverseFromEnd`)
    (:`Update`
      (`SceneComponent.K2_SetRelativeRotation` (`self.fridgedoor`) (`KismetMathLibrary.MakeRotator` 0.0 0.0 _angle) false false))))

(event `self.ReceiveBeginPlay`
  ; Fait apparaitre de la nourriture dans le frigo
  (`self.SpawnFood`))

(event `StartCountdown`)

(fn `SpawnFood`
  ; Détermine la Position/Type de nourriture
  (bind _returnvalue (`|SpawnActorFromClass` "/Game/MyContent/BP/Food/BP_Food.BP_Food_C" (`KismetMathLibrary.MakeTransform` (`SceneComponent.K2_GetComponentLocation` (`self.SpawnFood1`))) "Undefined" "MultiplyWithRoot" null null))
  (set `/Game/MyContent/BP/Food/BP_Master_item.FrigoREF` self _returnvalue))

(fn `UserConstructionScript`)