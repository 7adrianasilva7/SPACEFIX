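; BP_Master_holo is an interactable hologram actor that opens the UI_Hologram widget when the player interacts with it.
; Hover events toggle a custom depth and stencil outline on its StaticMesh, along with the interaction indicator on the player's PlayerEatREF.
; Interaction hides that indicator, creates the widget in the viewport and flags the hologram as read.
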(event `self.OnHovered`
  (params (IsHovered :type Boolean) (PlayerREF :type "/Game/FirstPerson/Blueprints/BP_FirstPersonCharacter Object Reference"))
  ; Interface d'événement
  (`/Engine/EditorBlueprintResources/StandardMacros.IsValid` PlayerREF
    (:`Is Valid`
      (`self.ToogleOutline` IsHovered)
      (`/Game/MyContent/UI/Tooltip/UI_Interagir.Toggle Interaction Indicator` (`/Game/FirstPerson/Blueprints/BP_FirstPersonCharacter.Player_Eat_REF` PlayerREF) IsHovered))))

(event `self.OnInteracted`
  (params (PlayerREF :type "/Game/FirstPerson/Blueprints/BP_FirstPersonCharacter Object Reference"))
  ; Interface d'événement
  (`/Engine/EditorBlueprintResources/StandardMacros.IsValid` PlayerREF
    (:`Is Valid`
      (`/Game/MyContent/UI/Tooltip/UI_Interagir.Toggle Interaction Indicator` (`/Game/FirstPerson/Blueprints/BP_FirstPersonCharacter.Player_Eat_REF` PlayerREF) false)
      (bind _returnvalue (`|CreateWidget` "/Game/MyContent/UI/Tutoriel/UI_Hologram.UI_Hologram_C"))
      (`UserWidget.AddToViewport` _returnvalue 0)
      (set `self.IsRead` true))))

(fn `ToogleOutline`
  (params (IsVisible :type Boolean))
  (bind _staticmesh (`self.StaticMesh`))
  (`PrimitiveComponent.SetRenderCustomDepth` _staticmesh IsVisible)
  (`PrimitiveComponent.SetCustomDepthStencilValue` _staticmesh (`KismetMathLibrary.SelectInt` 1 0 IsVisible)))

(fn `UserConstructionScript`)