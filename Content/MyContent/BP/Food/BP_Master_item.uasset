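; BP_Master_item is a food item actor that the player eats to restore hunger.
; Hover events toggle a custom depth stencil outline on its mesh and the interaction indicator on the player's PlayerEatREF.
; Interacting hides the indicator, restores the first-person character's hunger and destroys the item.
; Before destruction, it sets a delayed SpawnFood timer on the referenced fridge (FrigoREF) so food respawns there.
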(event `/Game/MyContent/Interface/BI_Interaction.OnHovered`
  (params (IsHovered :type Boolean) (PlayerREF :type "/Game/FirstPerson/Blueprints/BP_FirstPersonCharacter Object Reference"))
  ; Interface d'événement
  (`/Engine/EditorBlueprintResources/StandardMacros.IsValid` PlayerREF
    (:`Is Valid`
      (`self.ToggleOutline` IsHovered)
      (`/Game/MyContent/UI/Tooltype/UI_Interagir.Toggle Interaction Indicator` (`/Game/FirstPerson/Blueprints/BP_FirstPersonCharacter.Player_Eat_REF` PlayerREF) IsHovered))))

(event `/Game/MyContent/Interface/BI_Interaction.OnInteracted`
  (params (PlayerREF :type "/Game/FirstPerson/Blueprints/BP_FirstPersonCharacter Object Reference"))
  ; Interface d'événement
  (`/Engine/EditorBlueprintResources/StandardMacros.IsValid` PlayerREF
    (:`Is Valid`
      (`/Game/MyContent/UI/Tooltype/UI_Interagir.Toggle Interaction Indicator` (`/Game/FirstPerson/Blueprints/BP_FirstPersonCharacter.Player_Eat_REF` PlayerREF) false)
      (bind _asbp_first_person_character (cast `/Game/FirstPerson/Blueprints/BP_FirstPersonCharacter` (`GameplayStatics.GetPlayerCharacter` 0)))
      ;; Fait réapparaître la nourriture dans le frigo.
      (`KismetSystemLibrary.K2_SetTimer` (`self.FrigoREF`) "SpawnFood" 5.0)
      (`/Game/FirstPerson/Blueprints/BP_FirstPersonCharacter.Restore40Hunger` _asbp_first_person_character null)
      (`self.K2_DestroyActor`))))

(fn `ToggleOutline`
  (params (IsVisible :type Boolean))
  (bind _staticmesh (`self.StaticMesh`))
  (`PrimitiveComponent.SetRenderCustomDepth` _staticmesh IsVisible)
  (`PrimitiveComponent.SetCustomDepthStencilValue` _staticmesh (`KismetMathLibrary.SelectInt` 1 0 IsVisible)))

(fn `UserConstructionScript`)