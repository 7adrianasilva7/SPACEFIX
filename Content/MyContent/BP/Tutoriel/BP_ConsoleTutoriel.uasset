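; BP_ConsoleTutoriel is a tutorial console that shows a spinning satellite hologram and a confirmation text.
; Tick keeps rotating the hologram; LaunchAnim hides it and the ray, then a timeline types the feedback phrase out letter by letter using a growing substring.
; Three seconds after the typing ends, it clears the text and sets the linked satellite's IsOnRail flag to false.
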(event `self.ReceiveTick`
  (params (DeltaSeconds :type "Float (single-precision)"))
  (`SceneComponent.K2_AddLocalRotation` (`self.Hologramme_Sat`) (`KismetMathLibrary.MakeRotator` 0.0 (* DeltaSeconds 50.0)) false false))

(event `LaunchAnim`
  (`SceneComponent.SetVisibility` (`self.Hologramme_Sat`) false false)
  (`SceneComponent.SetVisibility` (`self.Rayon`) false false)
  (bind (_direction _alpha) (`Timeline|Timeline` :!via `PlayFromStart`)
    (:`Update`
      (`TextRenderComponent.K2_SetText` (`self.Confirmation`) (`KismetTextLibrary.Conv_StringToText` (`KismetStringLibrary.GetSubstring` (`self.PhraseFeedback`) 0 (`KismetMathLibrary.FTrunc` _alpha)))))
    (:`Finished`
      (`KismetSystemLibrary.Delay` 3.0)
      (`TextRenderComponent.K2_SetText` (`self.Confirmation`) "")
      (set `/Game/MyContent/BP/Tutoriel/BP_SatelliteTutoriel.IsOnRail` false (`self.LinkedSatellite`)))))

(fn `UserConstructionScript`)