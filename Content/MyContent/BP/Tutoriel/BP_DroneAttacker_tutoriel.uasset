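; Tutorial attack drone that turns toward the player within detection range and fires laser bursts.
; If visible shortly after BeginPlay, it fires once, then starts a looping burst timer after a random delay; each laser leads the player using velocity.
; TakeDamage flashes red and lowers HP; death spawns effects and teleports the drone away instead of destroying it.
; Tick restores visibility and collision whenever IsVisible is false, without resetting HP.
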(event `self.ReceiveBeginPlay`
  (`KismetSystemLibrary.Delay` 0.5)
  (if (`self.IsVisible?`)
    (`self.ShootAtPlayer`)
    (`|ExecutionSequence`
      (:`then_0`
        (`KismetSystemLibrary.Delay` (`KismetMathLibrary.RandomFloatInRange` 5.0 8.0))
        (`|ExecutionSequence`
          (:`then_0`
            (bind _asbp_first_person_character (cast `/Game/FirstPerson/Blueprints/BP_FirstPersonCharacter` (`GameplayStatics.GetPlayerCharacter` 0)))
            (set `self.Player` _asbp_first_person_character))
          (:`then_1`
            (`KismetSystemLibrary.K2_SetTimerDelegate` (delegate `ShootAtPlayer`) 3.0 true)))))))

(event `ShootAtPlayer`
  (`self.Laser`)
  (`KismetSystemLibrary.Delay` 0.2)
  (`self.Laser`)
  (`KismetSystemLibrary.Delay` 0.2)
  (`self.Laser`))

(event `self.ReceiveTick`
  (params (DeltaSeconds :type "Float (single-precision)"))
  (bind _hitzone (`self.HitZone`))
  (if (`self.IsVisible?`)
    (if (< (`self.GetDistanceTo` (`GameplayStatics.GetPlayerCharacter` 0)) (`self.DetectionRange`))
      (`self.K2_SetActorRotation` (`KismetMathLibrary.FindLookAtRotation` (`self.K2_GetActorLocation`) (`KismetMathLibrary.MakeVector` (.x (`self.K2_GetActorLocation` (`GameplayStatics.GetPlayerCharacter` 0))) (.y (`self.K2_GetActorLocation` (`GameplayStatics.GetPlayerCharacter` 0))) (+ (.z (`self.K2_GetActorLocation` (`GameplayStatics.GetPlayerCharacter` 0))) (`self.HoverHeight`))))))
    (else
      (`SceneComponent.SetVisibility` (`self.StaticMesh`) true false)
      (set `self.IsVisible?` true)
      (`PrimitiveComponent.SetCollisionEnabled` (`self.StaticMesh`) "QueryAndPhysics")
      (`PrimitiveComponent.SetCollisionEnabled` _hitzone "QueryAndPhysics")
      (`PrimitiveComponent.SetCollisionResponseToAllChannels` _hitzone "ECR_Block"))))

(fn `Laser`
  (bind _returnvalue (`GameplayStatics.GetPlayerCharacter` 0))
  (`|SpawnActorFromClass` "/Game/MyContent/BP/Drones/BP_LaserEnemy.BP_LaserEnemy_C" (`KismetMathLibrary.MakeTransform` (`self.K2_GetActorLocation`) (`KismetMathLibrary.FindLookAtRotation` (`self.K2_GetActorLocation`) (+ (`self.K2_GetActorLocation` _returnvalue) (`KismetMathLibrary.MakeVector` (* (.x (`self.GetVelocity` _returnvalue)) 0.3) (* (.y (`self.GetVelocity` _returnvalue)) 0.3) (* (.z (`self.GetVelocity` _returnvalue)) 0.3))))) "Undefined" "MultiplyWithRoot" null null))

(fn `ResetColor`
  (set `self.IsHit` false)
  (`PrimitiveComponent.SetMaterial` (`self.StaticMesh`) 0 "/Game/Fab/Futuristic_Surveillance_Drone_🛸/futuristic_surveillance_drone/Materials/Scene_-_Root.Scene_-_Root"))

(fn `ResetShoot`
  (set `self.CanShoot` true))

(fn `TakeDamage`
  (params (DamageAmount :type "Float (double-precision)"))
  (if (not (`self.IsHit`))
    (set `self.IsHit` true)
    (bind _returnvalue (`PrimitiveComponent.CreateDynamicMaterialInstance` (`self.StaticMesh`) 0 "/Game/MyContent/Materials/M_RedGlow.M_RedGlow" "None"))
    (`MaterialInstanceDynamic.SetVectorParameterValue` _returnvalue "BaseColor" (struct :`R` 10.0 :`A` 1.0))
    (`KismetSystemLibrary.K2_SetTimer` null "ResetColor" 0.1)
    (bind _output_get (set `self.HP` (`KismetMathLibrary.FClamp` (- (`self.HP`) DamageAmount) 0.0 100.0)))
    (if (<= _output_get 0.0)
      (`NiagaraFunctionLibrary.SpawnSystemAtLocation` "/Game/MyContent/NS/Drone/NS_DroneDead.NS_DroneDead" (+ (`self.K2_GetActorLocation`) (0.0 0.0 60.0)))
      (`GameplayStatics.PlaySoundAtLocation` "/Game/MyContent/SFX/explosionenemy.explosionenemy" (`SceneComponent.RelativeLocation` (`self.StaticMesh`)) (struct) 1.0 1.0 0.0 null null null null)
      (`SceneComponent.SetVisibility` (`self.StaticMesh`) true false)
      (set `self.IsVisible?` false)
      (`self.K2_SetActorLocation` (5000.0 5000.0 5000.0)))))

(fn `UserConstructionScript`)