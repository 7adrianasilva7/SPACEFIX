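; BP_Console_FinTutoriel is an end-of-tutorial console that validates a linked satellite once it has been delivered.
; An InteractionRange overlap sets IsReadyToValidate while the first-person character is inside.
; When ValidateSatellite is called in range with a delivered satellite, it launches that satellite's teleport, sets IsValidDoor and clears the ready flag.
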(event `self.InteractionRange.OnComponentBeginOverlap`
  (params (OverlappedComponent :type "PrimitiveComponent Object Reference") (OtherActor :type "Actor Object Reference") (OtherComp :type "PrimitiveComponent Object Reference") (OtherBodyIndex :type Integer) (bFromSweep :type Boolean) (SweepResult :type "HitResult Structure (by ref)"))
  (cast `/Game/FirstPerson/Blueprints/BP_FirstPersonCharacter` OtherActor)
  (set `self.IsReadyToValidate` true))

(event `self.InteractionRange.OnComponentEndOverlap`
  (params (OverlappedComponent :type "PrimitiveComponent Object Reference") (OtherActor :type "Actor Object Reference") (OtherComp :type "PrimitiveComponent Object Reference") (OtherBodyIndex :type Integer))
  (cast `/Game/FirstPerson/Blueprints/BP_FirstPersonCharacter` OtherActor)
  (set `self.IsReadyToValidate` false))

(event `ValidateSatellite`
  (bind _linkedsatellite (`self.LinkedSatellite`))
  (`/Engine/EditorBlueprintResources/StandardMacros.IsValid` _linkedsatellite
    (:`Is Valid`
      (if (and (`self.IsReadyToValidate`) (`/Game/MyContent/BP/Tutoriel/BP_SatelliteTutoriel.IsDelivered` _linkedsatellite))
        (`/Game/MyContent/BP/Tutoriel/BP_SatelliteTutoriel.LaunchTeleport` (`self.LinkedSatellite`))
        (set `self.IsValidDoor` true)
        (set `self.IsReadyToValidate` false)))))

(fn `UserConstructionScript`)