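; Tutorial satellite actor that travels along a rail toward a delivery target and can be switched to pickup mode.
; Tick moves it along world X while on an undamaged rail and not carried, flagging it delivered near the target.
; EnablePickupMode takes it off the rail and makes it pickupable.
; LaunchTeleport raises it with a timeline, then hides it, plays pop and Niagara effects, and destroys it.
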(event `self.ReceiveBeginPlay`
  (set `self.StartLocation` (`self.K2_GetActorLocation`)))

(event `self.ReceiveTick`
  (params (DeltaSeconds :type "Float (single-precision)"))
  (if (`self.IsCarriedByPlayer`)
    _
    (elif (and (`self.IsOnRail`) (not (`/Game/MyContent/BP/BP_Rail.IsRailDamaged` (`self.RailReference`))))
      (`self.K2_SetActorLocation` (+ (`self.K2_GetActorLocation`) (`KismetMathLibrary.MakeVector` (* (`self.MoveSpeed`) DeltaSeconds))))
      (if (< (`KismetMathLibrary.Vector_Distance` (`self.K2_GetActorLocation`) (`self.TargetLocation`)) 80.0)
        (set `self.IsOnRail` true)
        (set `self.IsDelivered` true)
        (`KismetSystemLibrary.PrintString` "est arrivé!")))))

(event `EnablePickupMode`
  (set `self.IsPickupable` true)
  (set `self.IsOnRail` false))

(event `LaunchTeleport`
  (bind _returnvalue (`self.K2_GetActorLocation`))
  (bind _returnvalue_2 (`self.K2_GetActorLocation`))
  (`GameplayStatics.SpawnSoundAtLocation` "/Game/MyContent/SFX/teleport.teleport" (`self.K2_GetActorLocation`) (struct) 1.0 1.0 0.0 null null)
  (bind (_direction _alpha) (`Timeline|Timeline` :!via `PlayFromStart`)
    (:`Update`
      (`self.K2_SetActorLocation` (`KismetMathLibrary.VLerp` _returnvalue (+ _returnvalue (0.0 0.0 20.0)) _alpha)))
    (:`Finished`
      (`SceneComponent.SetVisibility` (`self.SatelliteMesh`) false false)
      (`GameplayStatics.SpawnSoundAtLocation` "/Game/MyContent/SFX/pop.pop" _returnvalue_2 (struct) 1.0 1.0 0.0 null null)
      (`NiagaraFunctionLibrary.SpawnSystemAtLocation` "/Game/MyContent/NS/NS_SatelliteTeleport.NS_SatelliteTeleport" _returnvalue_2)
      (`self.K2_DestroyActor`))))

(fn `UserConstructionScript`)