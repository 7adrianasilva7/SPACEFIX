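; Tutorial copy of the main level's O2 drone, meant to appear only once as a shootable target.
; A one-time Box overlap reveals it, enables collision and sets full HP.
; TakeDamage flashes it red via a dynamic material and timer, then at zero HP plays death effects, hides it and disables collision.
; Generator seeking and attack startup remain in disconnected nodes, so BeginPlay and Tick do nothing and AttackGenerator's timer never starts.
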(event `self.ReceiveBeginPlay`
  ; Même drone que pour le niveau principal, mais apparait qu'une fois
)

(event `self.ReceiveTick`
  (params (DeltaSeconds :type "Float (single-precision)"))
  ; Même drone que pour le niveau principal, mais apparait qu'une fois
)

(event `self.Box.OnComponentBeginOverlap`
  (params (OverlappedComponent :type "PrimitiveComponent Object Reference") (OtherActor :type "Actor Object Reference") (OtherComp :type "PrimitiveComponent Object Reference") (OtherBodyIndex :type Integer) (bFromSweep :type Boolean) (SweepResult :type "HitResult Structure (by ref)"))
  (bind _hitzone (`self.HitZone`))
  ; Même drone que pour le niveau principal, mais apparait qu'une fois
  (`/Engine/EditorBlueprintResources/StandardMacros.DoOnce` false
    (:`Completed`
      (set `self.IsAttacking` false)
      (`SceneComponent.SetVisibility` (`self.DroneMesh`) true false)
      (set `self.IsVisible?` true)
      (`PrimitiveComponent.SetCollisionEnabled` (`self.DroneMesh`) "QueryAndPhysics")
      (`PrimitiveComponent.SetCollisionEnabled` _hitzone "QueryAndPhysics")
      (`PrimitiveComponent.SetCollisionResponseToAllChannels` _hitzone "ECR_Block")
      (set `self.HP` 100.0))))

(fn `AttackGenerator`
  (bind _attacksoundcomponent (`self.AttackSoundComponent`))
  (if (`self.IsVisible?`)
    (if (`self.IsAttacking`)
      (`/Game/MyContent/BP/Hunger_O2/BP_O2Generator.DamageGenerator` (`self.BP_O2GeneratorRef`))
      (if (not (`KismetSystemLibrary.IsValid` (`self.AttackSoundComponent`)))
        (bind _returnvalue (`GameplayStatics.SpawnSoundAtLocation` "/Game/MyContent/SFX/courtcircuit.courtcircuit" (`self.K2_GetActorLocation` (`self.BP_O2GeneratorRef`)) (struct) 1.0 1.0 0.0 null null))
        (set `self.AttackSoundComponent` _returnvalue))
      (elif (`KismetSystemLibrary.IsValid` _attacksoundcomponent)
        (`AudioComponent.Stop` _attacksoundcomponent)
        (set `self.AttackSoundComponent` null)))))

(fn `ResetColor`
  (set `self.IsHit` false)
  (`PrimitiveComponent.SetMaterial` (`self.DroneMesh`) 0 "/Game/Fab/Futuristic_Surveillance_Drone_🛸/futuristic_surveillance_drone/Materials/Scene_-_Root.Scene_-_Root"))

(fn `TakeDamage`
  (params (DamageAmount :type "Float (double-precision)"))
  (bind _hitzone (`self.HitZone`))
  (if (not (`self.IsHit`))
    (set `self.IsHit` true)
    (bind _returnvalue (`PrimitiveComponent.CreateDynamicMaterialInstance` (`self.DroneMesh`) 0 "/Game/MyContent/Materials/M_RedGlow.M_RedGlow" "None"))
    (`MaterialInstanceDynamic.SetVectorParameterValue` _returnvalue "BaseColor" (struct :`R` 10.0 :`A` 1.0))
    (`KismetSystemLibrary.K2_SetTimer` null "ResetColor" 0.1)
    (bind _output_get (set `self.HP` (`KismetMathLibrary.FClamp` (- (`self.HP`) DamageAmount) 0.0 100.0)))
    (if (<= _output_get 0.0)
      (`NiagaraFunctionLibrary.SpawnSystemAtLocation` "/Game/MyContent/NS/Drone/NS_DroneDead.NS_DroneDead" (+ (`self.K2_GetActorLocation`) (0.0 0.0 60.0)))
      (`GameplayStatics.PlaySoundAtLocation` "/Game/MyContent/SFX/explosionenemy.explosionenemy" (`SceneComponent.RelativeLocation` (`self.DroneMesh`)) (struct) 1.0 1.0 0.0 null null null null)
      (`|ExecutionSequence`
        (:`then_0`
          (bind _outactors (`GameplayStatics.GetAllActorsOfClass` "/Game/MyContent/BP/Satellite/BP_SpawnPoint.BP_SpawnPoint_C"))
          (for _array_element _outactors
            (if (< (`self.GetDistanceTo` null) 200.0)
              (set `/Game/MyContent/BP/Satellite/BP_SpawnPoint.IsOccupied` false _array_element)
              (`SceneComponent.SetVisibility` (`self.DroneMesh`) false false)
              (set `self.IsVisible?` false)
              (bind _asbp_first_person_character (cast `/Game/FirstPerson/Blueprints/BP_FirstPersonCharacter` (`GameplayStatics.GetPlayerCharacter` 0)))
              (set `/Game/FirstPerson/Blueprints/BP_FirstPersonCharacter.IsRepairing` false _asbp_first_person_character))))
        (:`then_1`
          (`SceneComponent.SetVisibility` (`self.DroneMesh`) false false)
          (set `self.IsVisible?` false)
          (`PrimitiveComponent.SetCollisionEnabled` (`self.DroneMesh`) "NoCollision")
          (`PrimitiveComponent.SetCollisionEnabled` _hitzone "NoCollision")
          (`PrimitiveComponent.SetCollisionResponseToAllChannels` _hitzone "ECR_Ignore"))))))

(fn `UserConstructionScript`)