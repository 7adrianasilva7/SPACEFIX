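; Enemy drone that seeks out the BP_O2Generator and damages it.
; Tick turns it toward the generator and moves it forward until within AttackRange, setting IsAttacking for a looping timer that deals damage and manages a short-circuit sound.
; TakeDamage flashes the mesh red, ignoring further hits until ResetColor.
; At zero HP it plays death effects, then frees a spawn point and destroys itself only if that loop's distance check passes.
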(event `self.ReceiveBeginPlay`
  (`|ExecutionSequence`
    (:`then_0`
      (bind _outactors (`GameplayStatics.GetAllActorsOfClass` "/Game/MyContent/BP/BP_O2Generator.BP_O2Generator_C"))
      (bind _output (`|GetArrayItem` _outactors))
      (`/Engine/EditorBlueprintResources/StandardMacros.IsValid` _output
        (:`Is Valid`
          (set `self.BP_O2GeneratorRef` _output))))
    (:`then_1`
      (`KismetSystemLibrary.K2_SetTimer` null "AttackGenerator" 1.0 true)
      (bind _returnvalue (`PrimitiveComponent.CreateDynamicMaterialInstance` (`/Game/MyContent/BP/BP_O2Generator.oxygen_tank` (`self.BP_O2GeneratorRef`)) 0 "/Game/Fab/SciFi_Style_Generator/scifi_style_generator/Materials/generator.generator" "None"))
      (set `self.DynMaterial` _returnvalue))))

(event `self.ReceiveTick`
  (params (DeltaSeconds :type "Float (single-precision)"))
  (`/Engine/EditorBlueprintResources/StandardMacros.IsValid` (`self.BP_O2GeneratorRef`)
    (:`Is Valid`
      (`self.K2_SetActorRotation` (`KismetMathLibrary.FindLookAtRotation` (`self.K2_GetActorLocation`) (`self.K2_GetActorLocation` (`self.BP_O2GeneratorRef`))))
      (if (> (`self.GetDistanceTo` (`self.BP_O2GeneratorRef`)) (`self.AttackRange`))
        (`self.AddMovementInput` (`self.GetActorForwardVector`))
        (set `self.IsAttacking` false)
        (else
          (set `self.IsAttacking` true))))
    (:`Is Not Valid`
      (bind _outactors (`GameplayStatics.GetAllActorsOfClass` "/Game/MyContent/BP/BP_O2Generator.BP_O2Generator_C"))
      (bind _output (`|GetArrayItem` _outactors))
      (`/Engine/EditorBlueprintResources/StandardMacros.IsValid` _output
        (:`Is Valid`
          (set `self.BP_O2GeneratorRef` _output))))))

(fn `AttackGenerator`
  (bind _attacksoundcomponent (`self.AttackSoundComponent`))
  (if (`self.IsAttacking`)
    (`/Game/MyContent/BP/BP_O2Generator.DamageGenerator` (`self.BP_O2GeneratorRef`))
    (if (not (`KismetSystemLibrary.IsValid` (`self.AttackSoundComponent`)))
      (bind _returnvalue (`GameplayStatics.SpawnSoundAtLocation` "/Game/MyContent/SFX/courtcircuit.courtcircuit" (`self.K2_GetActorLocation` (`self.BP_O2GeneratorRef`)) (struct) 1.0 1.0 0.0 null null))
      (set `self.AttackSoundComponent` _returnvalue))
    (elif (`KismetSystemLibrary.IsValid` _attacksoundcomponent)
      (`AudioComponent.Stop` _attacksoundcomponent)
      (set `self.AttackSoundComponent` null))))

(fn `ResetColor`
  (set `self.IsHit` false)
  (`PrimitiveComponent.SetMaterial` (`self.DroneMesh`) 0 "/Game/Fab/Futuristic_Surveillance_Drone_🛸/futuristic_surveillance_drone/Materials/Scene_-_Root.Scene_-_Root"))

(fn `TakeDamage`
  (params (DamageAmount :type "Float (double-precision)"))
  (if (not (`self.IsHit`))
    (set `self.IsHit` true)
    (bind _returnvalue (`PrimitiveComponent.CreateDynamicMaterialInstance` (`self.DroneMesh`) 0 "/Game/MyContent/Materials/M_RedGlow.M_RedGlow" "None"))
    (`MaterialInstanceDynamic.SetVectorParameterValue` _returnvalue "BaseColor" (struct :`R` 10.0 :`A` 1.0))
    (`KismetSystemLibrary.K2_SetTimer` null "ResetColor" 0.1)
    (bind _output_get (set `self.HP` (`KismetMathLibrary.FClamp` (- (`self.HP`) DamageAmount) 0.0 100.0)))
    (if (<= _output_get 0.0)
      (`NiagaraFunctionLibrary.SpawnSystemAtLocation` "/Game/MyContent/NS/Drone/NS_DroneDead.NS_DroneDead" (+ (`self.K2_GetActorLocation`) (0.0 0.0 60.0)))
      (`GameplayStatics.PlaySoundAtLocation` "/Game/MyContent/SFX/explosionenemy.explosionenemy" (`SceneComponent.RelativeLocation` (`self.DroneMesh`)) (struct) 1.0 1.0 0.0 null null null null)
      (bind _outactors (`GameplayStatics.GetAllActorsOfClass` "/Game/MyContent/BP/BP_SpawnPoint.BP_SpawnPoint_C"))
      (for _array_element _outactors
        (if (< (`self.GetDistanceTo` null) 200.0)
          (set `/Game/MyContent/BP/BP_SpawnPoint.IsOccupied` false _array_element)
          (`self.K2_DestroyActor`))))))

(fn `UserConstructionScript`)