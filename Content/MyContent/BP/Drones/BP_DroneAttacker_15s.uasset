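; Attacker drone enemy that faces the player within detection range and moves toward them through its AI controller.
; While visible, a looping timer fires three-laser bursts aimed ahead of the player using their velocity.
; Damage flashes the mesh red; at zero HP it plays death effects, frees nearby spawn points and hides itself if one is found.
; Tick makes a hidden drone visible again after 15 seconds, without restoring HP.
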(event `self.ReceiveBeginPlay`
  (`|ExecutionSequence`
    (:`then_0`
      (bind _asbp_first_person_character (cast `/Game/FirstPerson/Blueprints/BP_FirstPersonCharacter` (`GameplayStatics.GetPlayerCharacter` 0)))
      (set `self.Player` _asbp_first_person_character))
    (:`then_1`
      (`KismetSystemLibrary.K2_SetTimerDelegate` (delegate `ShootAtPlayer`) 2.0 true))))

(event `ShootAtPlayer`
  (if (`self.IsVisible?`)
    (`self.Laser`)
    (`KismetSystemLibrary.Delay` 0.2)
    (`self.Laser`)
    (`KismetSystemLibrary.Delay` 0.2)
    (`self.Laser`)))

(event `self.ReceiveTick`
  (params (DeltaSeconds :type "Float (single-precision)"))
  (bind _returnvalue (`self.K2_GetActorLocation` (`GameplayStatics.GetPlayerCharacter` 0)))
  (bind _returnvalue_2 (`self.GetDistanceTo` (`GameplayStatics.GetPlayerCharacter` 0)))
  (if (`self.IsVisible?`)
    (if (< _returnvalue_2 (`self.DetectionRange`))
      (`self.K2_SetActorRotation` (`KismetMathLibrary.FindLookAtRotation` (`self.K2_GetActorLocation`) (`KismetMathLibrary.MakeVector` (.x _returnvalue) (.y _returnvalue) (+ (.z _returnvalue) (`self.HoverHeight`)))))
      (if (> _returnvalue_2 700.0)
        (bind _asbp_drone_aicontroller (cast `/Game/MyContent/BP/BP_DroneAIController` (`AIBlueprintHelperLibrary.GetAIController` null)))
        (`AIController.MoveToLocation` _asbp_drone_aicontroller _returnvalue 700.0 true true false true null true)))
    (else
      (`KismetSystemLibrary.Delay` 15.0)
      (`SceneComponent.SetVisibility` (`self.StaticMesh`) true false)
      (set `self.IsVisible?` true))))

(fn `Laser`
  (bind _returnvalue (`GameplayStatics.GetPlayerCharacter` 0))
  (`|SpawnActorFromClass` "/Game/MyContent/BP/Drones/BP_LaserEnemy.BP_LaserEnemy_C" (`KismetMathLibrary.MakeTransform` (`self.K2_GetActorLocation`) (`KismetMathLibrary.FindLookAtRotation` (`self.K2_GetActorLocation`) (+ (`self.K2_GetActorLocation` _returnvalue) (`KismetMathLibrary.MakeVector` (* (.x (`self.GetVelocity` _returnvalue)) 0.3) (* (.y (`self.GetVelocity` _returnvalue)) 0.3) (* (.z (`self.GetVelocity` _returnvalue)) 0.3))))) "Undefined" "MultiplyWithRoot" null null))

(fn `ResetColor`
  (set `self.IsHit` false)
  (`PrimitiveComponent.SetMaterial` (`self.StaticMesh`) 0 "/Game/Fab/Futuristic_Surveillance_Drone_🛸/futuristic_surveillance_drone/Materials/Scene_-_Root.Scene_-_Root"))

(fn `ResetShoot`
  (set `self.CanShoot` true))

(fn `TakeDamage`
  (params (DamageAmount :type "Float (double-precision)"))
  (if (not (`self.IsHit`))
    (set `self.IsHit` true)
    (bind _returnvalue (`PrimitiveComponent.CreateDynamicMaterialInstance` (`self.StaticMesh`) 0 "/Game/MyContent/Materials/M_RedGlow.M_RedGlow" "None"))
    (`MaterialInstanceDynamic.SetVectorParameterValue` _returnvalue "BaseColor" (struct :`R` 10.0 :`A` 1.0))
    (`KismetSystemLibrary.K2_SetTimer` null "ResetColor" 0.1)
    (bind _output_get (set `self.HP` (`KismetMathLibrary.FClamp` (- (`self.HP`) DamageAmount) 0.0 100.0)))
    (if (<= _output_get 0.0)
      (`NiagaraFunctionLibrary.SpawnSystemAtLocation` "/Game/MyContent/NS/Drone/NS_DroneDead.NS_DroneDead" (+ (`self.K2_GetActorLocation`) (0.0 0.0 60.0)))
      (`GameplayStatics.PlaySoundAtLocation` "/Game/MyContent/SFX/explosionenemy.explosionenemy" (`SceneComponent.RelativeLocation` (`self.StaticMesh`)) (struct) 1.0 1.0 0.0 null null null null)
      (bind _outactors (`GameplayStatics.GetAllActorsOfClass` "/Game/MyContent/BP/BP_SpawnPoint.BP_SpawnPoint_C"))
      (for _array_element _outactors
        (if (< (`self.GetDistanceTo` null) 200.0)
          (set `/Game/MyContent/BP/BP_SpawnPoint.IsOccupied` false _array_element)
          (`SceneComponent.SetVisibility` (`self.StaticMesh`) false false)
          (set `self.IsVisible?` false))))))

(fn `UserConstructionScript`)