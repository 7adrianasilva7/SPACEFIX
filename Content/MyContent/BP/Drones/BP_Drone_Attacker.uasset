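; Enemy attack drone that chases the player, fires laser bursts and explodes when its HP runs out.
; Tick turns it toward a hover point above the player within detection range and moves it forward until it is close.
; A looping timer, independent of range, fires three-shot bursts of BP_LaserEnemy, leading the aim by player velocity.
; TakeDamage reduces clamped HP, then spawns death effects and destroys the actor at zero.
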(event `self.ReceiveBeginPlay`
  (`KismetSystemLibrary.K2_SetTimerDelegate` (delegate `ShootAtPlayer`) 2.0 true))

(event `ShootAtPlayer`
  (`self.Laser`)
  (`KismetSystemLibrary.Delay` 0.2)
  (`self.Laser`)
  (`KismetSystemLibrary.Delay` 0.2)
  (`self.Laser`))

(event `self.ReceiveTick`
  (params (DeltaSeconds :type "Float (single-precision)"))
  (bind _returnvalue (`self.GetDistanceTo` (`GameplayStatics.GetPlayerCharacter` 0)))
  (if (< _returnvalue (`self.DetectionRange`))
    (`self.K2_SetActorRotation` (`KismetMathLibrary.FindLookAtRotation` (`self.K2_GetActorLocation`) (`KismetMathLibrary.MakeVector` (.x (`self.K2_GetActorLocation` (`GameplayStatics.GetPlayerCharacter` 0))) (.y (`self.K2_GetActorLocation` (`GameplayStatics.GetPlayerCharacter` 0))) (+ (.z (`self.K2_GetActorLocation` (`GameplayStatics.GetPlayerCharacter` 0))) (`self.HoverHeight`)))))
    (if (> _returnvalue 700.0)
      (`self.AddMovementInput` (`self.GetActorForwardVector`) 0.5))))

(fn `Laser`
  (bind _returnvalue (`GameplayStatics.GetPlayerCharacter` 0))
  (`|SpawnActorFromClass` "/Game/MyContent/BP/Drones/BP_LaserEnemy.BP_LaserEnemy_C" (`KismetMathLibrary.MakeTransform` (`self.K2_GetActorLocation`) (`KismetMathLibrary.FindLookAtRotation` (`self.K2_GetActorLocation`) (+ (`KismetMathLibrary.MakeVector` (.x (`self.K2_GetActorLocation` _returnvalue)) (.y (`self.K2_GetActorLocation` _returnvalue)) (+ (.z (`self.K2_GetActorLocation` _returnvalue)) 40.0)) (`KismetMathLibrary.MakeVector` (* (.x (`self.GetVelocity` _returnvalue)) 0.3) (* (.y (`self.GetVelocity` _returnvalue)) 0.3) (* (.z (`self.GetVelocity` _returnvalue)) 0.3))))) "Undefined" "MultiplyWithRoot" null null))

(fn `ResetShoot`
  (set `self.CanShoot` true))

(fn `TakeDamage`
  (params (DamageAmount :type "Float (double-precision)"))
  (bind _output_get (set `self.HP` (`KismetMathLibrary.FClamp` (- (`self.HP`) DamageAmount) 0.0 100.0)))
  (if (<= _output_get 0.0)
    (`NiagaraFunctionLibrary.SpawnSystemAtLocation` "/Game/MyContent/NS/Drone/NS_DroneDead.NS_DroneDead" (+ (`self.K2_GetActorLocation`) (0.0 0.0 60.0)))
    (`GameplayStatics.PlaySoundAtLocation` "/Game/MyContent/SFX/explosionenemy.explosionenemy" (`SceneComponent.RelativeLocation` (`self.StaticMesh`)) (struct) 1.0 1.0 0.0 null null null null)
    (`self.K2_DestroyActor`)))

(fn `UserConstructionScript`)