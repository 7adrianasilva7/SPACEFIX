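; BP_DroneThief is an enemy drone that steals the satellite and flies it toward the nearest SAS.
; Tick steers it to the satellite; within attack range it takes it off its rail, waits, attaches it underneath, then picks the closest of three SAS actors to hover toward.
; At zero HP, only a carrying drone drops the satellite in pickup mode, makes start points blink, explodes and is destroyed.
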(event `self.ReceiveTick`
  (params (DeltaSeconds :type "Float (single-precision)"))
  (bind _bp_satellite_ref (`self.BP_Satellite_Ref`))
  (if (`self.HasSatellite`)
    (`/Engine/EditorBlueprintResources/StandardMacros.IsValid` (`self.TargetSAS`)
      (:`Is Valid`
        (`self.K2_SetActorRotation` (`KismetMathLibrary.FindLookAtRotation` (`self.K2_GetActorLocation`) (`KismetMathLibrary.MakeVector` (.x (`self.K2_GetActorLocation` (`self.TargetSAS`))) (.y (`self.K2_GetActorLocation` (`self.TargetSAS`))) (+ (.z (`self.K2_GetActorLocation` (`self.TargetSAS`))) (`self.HoverHeight`)))))
        (`self.AddMovementInput` (`self.GetActorForwardVector`)))
      (:`Is Not Valid`
        (`self.FindNearestSAS`)))
    (else
      (`/Engine/EditorBlueprintResources/StandardMacros.IsValid` _bp_satellite_ref
        (:`Is Valid`
          (if (and (not (`self.IsPickingUp`)) (not (`/Game/MyContent/BP/BP_Satellite.IsDelivered` _bp_satellite_ref)))
            (`self.K2_SetActorRotation` (`KismetMathLibrary.FindLookAtRotation` (`self.K2_GetActorLocation`) (`self.K2_GetActorLocation` (`self.BP_Satellite_Ref`))))
            (if (> (`self.GetDistanceTo` (`self.BP_Satellite_Ref`)) (`self.AttackRange`))
              (`self.AddMovementInput` (`self.GetActorForwardVector`))
              (elif (not (`self.IsPickingUp`))
                (`self.StartPickup`)))))))))

(event `StartPickup`
  (bind _bp_satellite_ref (`self.BP_Satellite_Ref`))
  (set `self.IsPickingUp` true)
  (set `/Game/MyContent/BP/BP_Satellite.IsOnRail` false (`self.BP_Satellite_Ref`))
  (`KismetSystemLibrary.Delay` 3.0)
  (set `self.HasSatellite` true)
  (set `self.IsPickingUp` false)
  (`self.K2_AttachToActor` _bp_satellite_ref self "None" "KeepWorld" "KeepRelative" "KeepRelative" true)
  (`self.K2_SetActorRelativeLocation` _bp_satellite_ref (0.0 0.0 -80.0) false false)
  (`self.FindNearestSAS`))

(event `DropSatellite`
  (bind _bp_satellite_ref (`self.BP_Satellite_Ref`))
  (`self.K2_DetachFromActor` _bp_satellite_ref "KeepWorld" "KeepRelative" "KeepRelative")
  (`self.K2_SetActorLocation` _bp_satellite_ref (+ (`self.K2_GetActorLocation`) (`KismetMathLibrary.MakeVector` 0.0 0.0 -100.0)) false false)
  (`/Game/MyContent/BP/BP_Satellite.EnablePickupMode` (`self.BP_Satellite_Ref`))
  (bind _outactors (`GameplayStatics.GetAllActorsOfClass` "/Game/MyContent/BP/BP_StartPoint.BP_StartPoint_C"))
  (`/Game/MyContent/BP/BP_StartPoint.StartBlink` _outactors))

(event `FindNearestSAS`
  (bind _returnvalue (`self.GetDistanceTo` (`self.SAS1Ref`)))
  (bind _returnvalue_2 (`self.GetDistanceTo` (`self.SAS3Ref`)))
  (bind _returnvalue_3 (`self.GetDistanceTo` (`self.SAS2Ref`)))
  (if (< _returnvalue _returnvalue_3)
    (if (< _returnvalue _returnvalue_2)
      (set `self.TargetSAS` (`self.SAS1Ref`))
      (else
        (set `self.TargetSAS` (`self.SAS3Ref`))))
    (elif (< _returnvalue_3 _returnvalue_2)
      (set `self.TargetSAS` (`self.SAS2Ref`))
      (else
        (set `self.TargetSAS` (`self.SAS3Ref`))))))

(fn `TakeDamage`
  (params (DamageAmount :type "Float (double-precision)"))
  (bind _output_get (set `self.HP` (`KismetMathLibrary.FClamp` (- (`self.HP`) DamageAmount) 0.0 100.0)))
  (if (<= _output_get 0.0)
    (if (`self.HasSatellite`)
      (`self.DropSatellite`)
      (`NiagaraFunctionLibrary.SpawnSystemAtLocation` "/Game/MyContent/NS/Drone/NS_DroneDead.NS_DroneDead" (+ (`self.K2_GetActorLocation`) (0.0 0.0 60.0)))
      (`GameplayStatics.PlaySoundAtLocation` "/Game/MyContent/SFX/explosionenemy.explosionenemy" (`SceneComponent.RelativeLocation` (`self.StaticMesh`)) (struct) 1.0 1.0 0.0 null null null null)
      (`self.K2_DestroyActor`))))

(fn `UserConstructionScript`)