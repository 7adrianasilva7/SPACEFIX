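; Thief drone that stays hidden on the satellite and, once the player has delivered two, appears after random delays to steal it.
; While visible it halts the satellite's rail movement and fills a player-facing steal bar, triggering the game-over screen when full.
; Damage flashes it red; at zero HP it explodes, hides for reuse and puts the satellite back on rail.
; Older chase and carry-to-airlock logic remains, mostly disconnected.
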(event `self.ReceiveBeginPlay`
  (bind _hitzone (`self.HitZone`))
  ;[0.4678 0.06938 0.0933] Point d'apparition du drone
  ;;[0 0.4678 0.4601] Set le temps de la time line
  (`|ExecutionSequence`
    (:`then_0`
      (set `self.Time` 0.0)
      (`self.Position du satellite`)
      (`SceneComponent.SetVisibility` (`self.StaticMesh`) false false)
      (set `self.IsVisible?` false)
      (`KismetSystemLibrary.Delay` (`KismetMathLibrary.RandomFloatInRange` 2.0 3.0))
      (bind _outactors (`GameplayStatics.GetAllActorsOfClass` "/Game/MyContent/BP/BP_Satellite.BP_Satellite_C"))
      (bind _output (`|GetArrayItem` _outactors))
      (`/Engine/EditorBlueprintResources/StandardMacros.IsValid` _output
        (:`Is Valid`
          (set `self.BP_Satellite_Ref` _output))))
    (:`then_1`
      (`PrimitiveComponent.SetCollisionEnabled` _hitzone "NoCollision")
      (`PrimitiveComponent.SetCollisionResponseToAllChannels` _hitzone "ECR_Ignore"))
    (:`then_2`
      (cast `/Game/FirstPerson/Blueprints/BP_FirstPersonCharacter` (`GameplayStatics.GetPlayerCharacter` 0))
      (bind _returnvalue (`|CreateWidget` "/Game/MyContent/UI/UI_StealFeedback.UI_StealFeedback_C"))
      (`Widget.SetVisibility` _returnvalue "Hidden")
      (bind _output_get (set `self.ui_steal-feedback` _returnvalue))
      (`UserWidget.AddToViewport` _output_get 0))))

(event `self.ReceiveTick`
  (params (DeltaSeconds :type "Float (single-precision)"))
  (bind _widget (`self.Widget`))
  ;[0.4678 0.06938 0.0933] Fonctionnement du drone
  (`|ExecutionSequence`
    (:`then_0`
      (bind _outactors (`GameplayStatics.GetAllActorsOfClass` "/Game/MyContent/BP/BP_Satellite.BP_Satellite_C"))
      (bind _output (`|GetArrayItem` _outactors))
      (`/Engine/EditorBlueprintResources/StandardMacros.IsValid` _output
        (:`Is Valid`
          (set `self.BP_Satellite_Ref` _output)
          (bind _asbp_first_person_character (cast `/Game/FirstPerson/Blueprints/BP_FirstPersonCharacter` (`GameplayStatics.GetPlayerCharacter` 0)))
          (if (>= (`/Game/FirstPerson/Blueprints/BP_FirstPersonCharacter.SatellitesDelivered` _asbp_first_person_character) 2)
            (if (`self.IsVisible?`)
              ;;[0 0.4678 0.4601] Quand la Progress Bar est complete, le GameOver se lance
              (`self.Lancement GameOver`)
              (else
                ;;[0 0.4678 0.4601] Temps d'apparition
                (`KismetSystemLibrary.Delay` (`KismetMathLibrary.RandomFloatInRange` 8.0 12.0))
                (`self.Apparition drone`)
                (`Widget.SetVisibility` (`self.ui_steal-feedback`) "Visible")))))))
    (:`then_1`
      ;;[0 0.4678 0.4601] Système de Progress Bar
      (if (`self.IsVisible?`)
        (`SceneComponent.SetVisibility` _widget true false)
        (bind _asui_steal_bar (cast `/Game/MyContent/UI/UI_StealBar` (`WidgetComponent.GetUserWidgetObject` _widget)))
        (bind _output_get (set `self.Time` (`KismetMathLibrary.FClamp` (+ (* (/ (`GameplayStatics.GetWorldDeltaSeconds`) 10.0) (`self.Steal`)) (`self.Time`)))))
        (`ProgressBar.SetPercent` (`/Game/MyContent/UI/UI_StealBar.PB_Repair` _asui_steal_bar) _output_get)
        (set `/Game/MyContent/BP/BP_Satellite.IsOnRail` false (`self.BP_Satellite_Ref`))
        (else
          (`SceneComponent.SetVisibility` _widget false false))))
    (:`then_2`
      ;;[0 0.4678 0.4601] Garde la position du satelite
      (`self.Position du satellite`))
    (:`then_3`
      ;[0.4678 0.06938 0.0933] Apparition de la Progress Bar + distance d'affichage
      (if (`self.IsVisible?`)
        (if (<= (`self.GetDistanceTo` (`GameplayStatics.GetPlayerCharacter` 0)) 2500.0)
          (`SceneComponent.SetVisibility` (`self.Widget`) true false)
          (`SceneComponent.K2_SetWorldRotation` (`self.Widget`) (`KismetMathLibrary.FindLookAtRotation` (`self.K2_GetActorLocation`) (`PlayerCameraManager.GetCameraLocation` (`GameplayStatics.GetPlayerCameraManager` 0))) false false)
          (else
            (`SceneComponent.SetVisibility` (`self.Widget`) false false)))))))

(event `DropSatellite`
  (bind _bp_satellite_ref (`self.BP_Satellite_Ref`))
  ;[0.04519 0.016 0.02624] Ancien code
  (set `/Game/MyContent/BP/BP_Satellite.IsOnRail` false _bp_satellite_ref)
  (`self.K2_DetachFromActor` _bp_satellite_ref "KeepWorld" "KeepRelative" "KeepRelative")
  (`self.K2_SetActorLocation` _bp_satellite_ref (+ (`self.K2_GetActorLocation`) (`KismetMathLibrary.MakeVector` 0.0 0.0 -100.0)) false false)
  (`GameplayStatics.PlaySound2D` "/Game/MyContent/SFX/Robot/Drop1.Drop1" 0.8 1.5 0.0 null null)
  (`/Game/MyContent/BP/BP_Satellite.EnablePickupMode` (`self.BP_Satellite_Ref`))
  (bind _outactors (`GameplayStatics.GetAllActorsOfClass` "/Game/MyContent/BP/BP_StartPoint.BP_StartPoint_C"))
  (`/Game/MyContent/BP/BP_StartPoint.ShowDepositEffect` (`|GetArrayItem` _outactors)))

(event `FindNearestSAS`
  ;[0.04519 0.016 0.02624] Ancien code
)

(event `StartPickup`
  (bind _bp_satellite_ref (`self.BP_Satellite_Ref`))
  ;[0.4678 0.06938 0.0933] Créer le GameOver
  (`/Engine/EditorBlueprintResources/StandardMacros.DoOnce` false
    (:`Completed`
      (`/Engine/EditorBlueprintResources/StandardMacros.IsValid` _bp_satellite_ref
        (:`Is Valid`
          (set `self.IsPickingUp` true)
          (set `/Game/MyContent/BP/BP_Satellite.IsOnRail` false _bp_satellite_ref)
          (`GameplayStatics.PlaySound2D` "/Game/MyContent/SFX/Robot/Pick-up1.Pick-up1" 1.5 2.5 0.9 null null)
          (bind _returnvalue (`|CreateWidget` "/Game/MyContent/UI/GameOver/UI_BlackDeath_End.UI_BlackDeath_End_C"))
          (`UserWidget.AddToViewport` _returnvalue 0))))))

(fn `Apparition drone`
  (bind _hitzone (`self.HitZone`))
  (`SceneComponent.SetVisibility` (`self.StaticMesh`) true false)
  (set `self.IsVisible?` true)
  (`PrimitiveComponent.SetCollisionEnabled` (`self.StaticMesh`) "QueryAndPhysics")
  (`PrimitiveComponent.SetCollisionEnabled` _hitzone "QueryAndPhysics")
  (`PrimitiveComponent.SetCollisionResponseToAllChannels` _hitzone "ECR_Block")
  (set `self.HP` 100.0)
  (set `self.Time` 0.0))

(fn `CalculSAS`
  (returns (ReturnValue :type "Rotator Structure"))
  (return (`KismetMathLibrary.FindLookAtRotation` (`self.K2_GetActorLocation`) (`KismetMathLibrary.MakeVector` (.x (`self.K2_GetActorLocation` (`self.TargetSAS`))) (.y (`self.K2_GetActorLocation` (`self.TargetSAS`))) (+ (.z (`self.K2_GetActorLocation` (`self.TargetSAS`))) (`self.HoverHeight`))))))

(fn `Lancement GameOver`
  (if (>= (`self.Time`) 1.0)
    (`self.StartPickup`)))

(fn `NonVisible`
  (bind _hitzone (`self.HitZone`))
  (bind _staticmesh (`self.StaticMesh`))
  (set `self.IsVisible?` false)
  (set `self.IsPickingUp` false)
  (`PrimitiveComponent.SetCollisionEnabled` _hitzone "NoCollision")
  (`PrimitiveComponent.SetCollisionResponseToAllChannels` _hitzone "ECR_Ignore")
  (`SceneComponent.SetVisibility` (`self.StaticMesh`) false false)
  (`PrimitiveComponent.SetCollisionEnabled` _staticmesh "NoCollision")
  (`PrimitiveComponent.SetCollisionResponseToAllChannels` _staticmesh "ECR_Ignore"))

(fn `Position du satellite`
  (bind _bp_satellite_ref (`self.BP_Satellite_Ref`)
    (:`then`
      (`self.K2_SetActorLocation` (`KismetMathLibrary.MakeVector` (.x (`self.K2_GetActorLocation` _bp_satellite_ref)) (+ (.y (`self.K2_GetActorLocation` _bp_satellite_ref)) 90.0) (.z (`self.K2_GetActorLocation` _bp_satellite_ref)))))
    (:`else`)))

(fn `ResetColor`
  (set `self.IsHit` false)
  (`PrimitiveComponent.SetMaterial` (`self.StaticMesh`) 0 "/Game/Fab/Futuristic_Surveillance_Drone_🛸/futuristic_surveillance_drone/Materials/Scene_-_Root.Scene_-_Root"))

(fn `TakeDamage`
  (params (DamageAmount :type "Float (double-precision)"))
  (bind _hitzone (`self.HitZone`))
  (bind _bp_satellite_ref (`self.BP_Satellite_Ref`))
  (if (`self.IsVisible?`)
    (if (not (`self.IsHit`))
      (set `self.IsHit` true)
      (bind _returnvalue (`PrimitiveComponent.CreateDynamicMaterialInstance` (`self.StaticMesh`) 0 "/Game/MyContent/Materials/M_RedGlow.M_RedGlow" "None"))
      (`MaterialInstanceDynamic.SetVectorParameterValue` _returnvalue "BaseColor" (struct :`R` 10.0 :`A` 1.0))
      (`KismetSystemLibrary.K2_SetTimer` null "ResetColor" 0.1)
      (bind _output_get (set `self.HP` (`KismetMathLibrary.FClamp` (- (`self.HP`) DamageAmount) 0.0 100.0)))
      (if (<= _output_get 0.0)
        (`|ExecutionSequence`
          (:`then_0`
            (`NiagaraFunctionLibrary.SpawnSystemAtLocation` "/Game/MyContent/NS/Drone/NS_DroneDead.NS_DroneDead" (+ (`self.K2_GetActorLocation`) (0.0 0.0 60.0)))
            (`GameplayStatics.PlaySoundAtLocation` "/Game/MyContent/SFX/explosionenemy.explosionenemy" (`SceneComponent.RelativeLocation` (`self.StaticMesh`)) (struct) 1.0 1.0 0.0 null null null null))
          (:`then_1`
            (`/Engine/EditorBlueprintResources/StandardMacros.IsValid` _bp_satellite_ref
              (:`Is Valid`
                (`/Game/MyContent/BP/BP_Satellite.EnablePickupMode` _bp_satellite_ref)
                (bind _outactors (`GameplayStatics.GetAllActorsOfClass` "/Game/MyContent/BP/BP_SpawnPoint.BP_SpawnPoint_C"))
                (for _array_element _outactors
                  (if (< (`self.GetDistanceTo` null) 200.0)
                    (set `/Game/MyContent/BP/BP_SpawnPoint.IsOccupied` false _array_element)
                    (set `self.IsVisible?` false)
                    (`Widget.SetVisibility` (`self.ui_steal-feedback`) "Hidden"))))))
          (:`then_2`
            (`SceneComponent.SetVisibility` (`self.StaticMesh`) false false)
            (set `self.IsVisible?` false)
            (`PrimitiveComponent.SetCollisionEnabled` (`self.StaticMesh`) "NoCollision")
            (`PrimitiveComponent.SetCollisionEnabled` _hitzone "NoCollision")
            (`PrimitiveComponent.SetCollisionResponseToAllChannels` _hitzone "ECR_Ignore")
            (set `/Game/MyContent/BP/BP_Satellite.MoveSpeed` 150.0 (`self.BP_Satellite_Ref`))
            (set `/Game/MyContent/BP/BP_Satellite.IsOnRail` true (`self.BP_Satellite_Ref`))))))))

(fn `UserConstructionScript`)