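; BP_CockpitTrigger is a trigger zone that registers the delivery of a BP_Satellite when one overlaps it.
; The overlapping satellite is taken off its rail, marked as delivered, and a validation sound plays at its location.
; All BP_wall_lamp_E actors then blink green, with the BP_Wall_lamp_A blink loop nested inside, so it repeats for each E lamp.
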(event `self.TriggerZone.OnComponentBeginOverlap`
  (params (OverlappedComponent :type "PrimitiveComponent Object Reference") (OtherActor :type "Actor Object Reference") (OtherComp :type "PrimitiveComponent Object Reference") (OtherBodyIndex :type Integer) (bFromSweep :type Boolean) (SweepResult :type "HitResult Structure (by ref)"))
  (bind _asbp_satellite (cast `/Game/MyContent/BP/BP_Satellite` OtherActor))
  (set `/Game/MyContent/BP/BP_Satellite.IsOnRail` false _asbp_satellite)
  (set `/Game/MyContent/BP/BP_Satellite.IsDelivered` true _asbp_satellite)
  (`GameplayStatics.SpawnSoundAtLocation` "/Game/MyContent/SFX/validation.validation" (`self.K2_GetActorLocation` _asbp_satellite) (struct) 1.0 1.0 0.0 null null)
  (bind _outactors (`GameplayStatics.GetAllActorsOfClass` "/Game/MyContent/BP/BP_wall_lamp_E.BP_wall_lamp_E_C"))
  (for _array_element _outactors
    (`/Game/MyContent/BP/BP_wall_lamp_E.BlinkGreen` _array_element)
    (bind _outactors_2 (`GameplayStatics.GetAllActorsOfClass` "/Game/MyContent/BP/BP_Wall_lamp_A.BP_Wall_lamp_A_C"))
    (for _array_element_2 _outactors_2
      (`/Game/MyContent/BP/BP_Wall_lamp_A.BlinkGreen2` _array_element_2))))

(fn `UserConstructionScript`)