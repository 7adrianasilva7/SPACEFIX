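; Interactive console that shows a rotating satellite hologram and controls a linked satellite.
; A timeline animates the button press, while LaunchAnim hides the hologram and cone and types out feedback text by revealing a growing substring.
; Three seconds after the text finishes, it clears the text and sets the linked satellite's IsOnRail to false.
; ResetConsole restores the hologram and cone and clears both its activated flag and the player's HasPlayed flag.
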(event `ButtonPressTimeline`
  (bind (_direction _alpha) (`Timeline|ButtonPress` :!via `PlayFromStart`)
    (:`Update`
      (`SceneComponent.K2_SetRelativeLocation` (`self.Button`) (`KismetMathLibrary.MakeVector` 0.0 46.22593 (+ _alpha 79.323203)) false false))))

(event `self.ReceiveTick`
  (params (DeltaSeconds :type "Float (single-precision)"))
  (`SceneComponent.K2_AddLocalRotation` (`self.Hologramme_Sat`) (`KismetMathLibrary.MakeRotator` 0.0 (* DeltaSeconds 50.0)) false false))

(event `LaunchAnim`
  (bind _linkedsatellite (`self.LinkedSatellite`))
  (`SceneComponent.SetVisibility` (`self.Hologramme_Sat`) false false)
  (`SceneComponent.SetVisibility` (`self.Cône`) false false)
  (bind (_direction _alpha) (`Timeline|Timeline` :!via `PlayFromStart`)
    (:`Update`
      (`TextRenderComponent.K2_SetText` (`self.Confirmation`) (`KismetTextLibrary.Conv_StringToText` (`KismetStringLibrary.GetSubstring` (`self.PhraseFeedback`) 0 (`KismetMathLibrary.FTrunc` _alpha)))))
    (:`Finished`
      (`KismetSystemLibrary.Delay` 3.0)
      (`TextRenderComponent.K2_SetText` (`self.Confirmation`) "")
      (`/Engine/EditorBlueprintResources/StandardMacros.IsValid` _linkedsatellite
        (:`Is Valid`
          (set `/Game/MyContent/BP/BP_Satellite.IsOnRail` false _linkedsatellite))))))

(event `ResetConsole`
  (`SceneComponent.SetVisibility` (`self.Hologramme_Sat`) true false)
  (`SceneComponent.SetVisibility` (`self.Cône`) true false)
  (set `self.IsActivated` false)
  (bind _asbp_first_person_character (cast `/Game/FirstPerson/Blueprints/BP_FirstPersonCharacter` (`GameplayStatics.GetPlayerCharacter` 0)))
  (set `/Game/FirstPerson/Blueprints/BP_FirstPersonCharacter.HasPlayed` false _asbp_first_person_character))

(fn `UserConstructionScript`)