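; BP_Generator is a generator that can be broken and repaired, tracking its state in an IsBroken flag.
; Its TakeDamage event sets the flag, and its Repairing event clears it only when the generator is broken.
; Both events cast player 0's character to BP_FirstPersonCharacter and mirror the state into that character's IsGeneratorBroken variable.
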(event `TakeDamage`
  (set `self.bIsBroken` true)
  (bind _asbp_first_person_character (cast `/Game/FirstPerson/Blueprints/BP_FirstPersonCharacter` (`GameplayStatics.GetPlayerCharacter` 0)))
  (set `/Game/FirstPerson/Blueprints/BP_FirstPersonCharacter.bIsGeneratorBroken` true _asbp_first_person_character))

(event `Repairing`
  (if (`self.bIsBroken`)
    (set `self.bIsBroken` false)
    (bind _asbp_first_person_character (cast `/Game/FirstPerson/Blueprints/BP_FirstPersonCharacter` (`GameplayStatics.GetPlayerCharacter` 0)))
    (set `/Game/FirstPerson/Blueprints/BP_FirstPersonCharacter.bIsGeneratorBroken` false _asbp_first_person_character)))

(fn `UserConstructionScript`)