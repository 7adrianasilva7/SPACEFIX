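; Wave manager that spawns attacker, O2 and thief drones, with caps and timings set by CurrentLevel on BeginPlay.
; StartWaves flags the satellite as launched, then starts a looping attacker timer and one-shot O2 and thief timers, the latter only if thieves are allowed.
; Each spawn function claims a free BP_SpawnPoint of matching SpawnType and increments its count, but spawns at the first spawn point found, not the claimed one.
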(event `self.ReceiveBeginPlay`
  (`self.SetLevelParameters`))

(event `StartWaves`
  (set `self.IsSatelliteLaunched` true)
  (`KismetSystemLibrary.K2_SetTimer` null "TrySpawnAttacker" (`self.SpawnInterval`) true)
  (`KismetSystemLibrary.K2_SetTimer` null "TrySpawnO2" (`self.O2SpawnDelay`))
  (if (> (`self.MaxThieves`) 0)
    (`KismetSystemLibrary.K2_SetTimer` null "TrySpawnThief" 20.0)))

(fn `SetLevelParameters`
  (switch `int` (`self.CurrentLevel`)
    (:`1`
      (set `self.MaxAttackers` 2)
      (set `self.MaxO2Drones` 1)
      (set `self.MaxThieves` 0)
      (set `self.SpawnInterval` 5.0)
      (set `self.O2SpawnDelay` 30.0))
    (:`2`
      (set `self.MaxAttackers` 4)
      (set `self.MaxO2Drones` 2)
      (set `self.MaxThieves` 1)
      (set `self.SpawnInterval` 4.0)
      (set `self.O2SpawnDelay` 25.0))
    (:`3`
      (set `self.MaxAttackers` 8)
      (set `self.MaxO2Drones` 2)
      (set `self.MaxThieves` 2)
      (set `self.SpawnInterval` 3.0)
      (set `self.O2SpawnDelay` 20.0))))

(fn `TrySpawnAttacker`
  (locals (SpawnedOne :type Boolean))
  (`KismetSystemLibrary.PrintString` "atk")
  (if (and (`self.IsSatelliteLaunched`) (< (`self.CurrentAttackers`) (`self.MaxAttackers`)))
    (bind _outactors (`GameplayStatics.GetAllActorsOfClass` "/Game/MyContent/BP/Satellite/BP_SpawnPoint.BP_SpawnPoint_C"))
    (set `local.SpawnedOne` false)
    (for _array_element _outactors
      (if (`local.SpawnedOne`)
        _
        (elif (and (not (`/Game/MyContent/BP/Satellite/BP_SpawnPoint.IsOccupied` _array_element)) (`KismetStringLibrary.EqualEqual_StrStr` (`/Game/MyContent/BP/Satellite/BP_SpawnPoint.SpawnType` _array_element) "Attacker"))
          (set `/Game/MyContent/BP/Satellite/BP_SpawnPoint.IsOccupied` true _array_element)
          (`|SpawnActorFromClass` "/Game/MyContent/BP/Drones/BP_DroneAttacker_.BP_DroneAttacker__C" (`KismetMathLibrary.MakeTransform` (`self.K2_GetActorLocation` (`|GetArrayItem` _outactors))) "Undefined" "MultiplyWithRoot" null null)
          (set `self.CurrentAttackers` (+ (`self.CurrentAttackers`) 1))
          (set `local.SpawnedOne` true))))))

(fn `TrySpawnO2`
  (locals (SpawnedOne :type Boolean))
  (`KismetSystemLibrary.PrintString` "o2")
  (if (< (`self.Current02Drones`) (`self.MaxO2Drones`))
    (bind _outactors (`GameplayStatics.GetAllActorsOfClass` "/Game/MyContent/BP/Satellite/BP_SpawnPoint.BP_SpawnPoint_C"))
    (set `local.SpawnedOne` false)
    (for _array_element _outactors
      (if (`local.SpawnedOne`)
        _
        (elif (and (not (`/Game/MyContent/BP/Satellite/BP_SpawnPoint.IsOccupied` _array_element)) (`KismetStringLibrary.EqualEqual_StrStr` (`/Game/MyContent/BP/Satellite/BP_SpawnPoint.SpawnType` _array_element) "O2"))
          (set `/Game/MyContent/BP/Satellite/BP_SpawnPoint.IsOccupied` true _array_element)
          (`|SpawnActorFromClass` "/Game/MyContent/BP/Drones/BP_DroneO2.BP_DroneO2_C" (`KismetMathLibrary.MakeTransform` (`self.K2_GetActorLocation` (`|GetArrayItem` _outactors))) "Undefined" "MultiplyWithRoot" null null)
          (set `self.Current02Drones` (+ (`self.Current02Drones`) 1))
          (set `local.SpawnedOne` true))))))

(fn `TrySpawnThief`
  (locals (SpawnedOne :type Boolean))
  (`KismetSystemLibrary.PrintString` "thief")
  (if (< (`self.CurrentThieves`) (`self.MaxThieves`))
    (bind _outactors (`GameplayStatics.GetAllActorsOfClass` "/Game/MyContent/BP/Satellite/BP_SpawnPoint.BP_SpawnPoint_C"))
    (set `local.SpawnedOne` false)
    (for _array_element _outactors
      (if (`local.SpawnedOne`)
        _
        (elif (and (not (`/Game/MyContent/BP/Satellite/BP_SpawnPoint.IsOccupied` _array_element)) (`KismetStringLibrary.EqualEqual_StrStr` (`/Game/MyContent/BP/Satellite/BP_SpawnPoint.SpawnType` _array_element) "Thief"))
          (set `/Game/MyContent/BP/Satellite/BP_SpawnPoint.IsOccupied` true _array_element)
          (`|SpawnActorFromClass` "/Game/MyContent/BP/Drones/BP_DroneThiefSafe.BP_DroneThiefSafe_C" (`KismetMathLibrary.MakeTransform` (`self.K2_GetActorLocation` (`|GetArrayItem` _outactors))) "Undefined" "MultiplyWithRoot" null null)
          (set `self.CurrentThieves` (+ (`self.CurrentThieves`) 1))
          (set `local.SpawnedOne` true))))))

(fn `UserConstructionScript`)