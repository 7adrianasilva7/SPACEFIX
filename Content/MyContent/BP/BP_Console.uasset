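; BP_Console is an in-game console that lets the player launch a linked satellite.
; Showing the console creates a UI_Console widget owned by it, switches input to UI-only and shows the cursor.
; Launching marks the console activated, sets the linked satellite's IsOnRail flag, and restores game-only input with the cursor hidden.
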(event `ShowConsoleUI`
  (bind _returnvalue (`GameplayStatics.GetPlayerController` 0))
  (bind _returnvalue_2 (`|CreateWidget` "/Game/MyContent/UI/UI_Console.UI_Console_C"))
  (set `/Game/MyContent/UI/UI_Console.OwnerConsole` self _returnvalue_2)
  (`UserWidget.AddToViewport` _returnvalue_2 0)
  (`WidgetBlueprintLibrary.SetInputMode_UIOnlyEx` _returnvalue _returnvalue_2)
  (set `PlayerController.bShowMouseCursor` true _returnvalue))

(event `LaunchSatellite`
  (bind _returnvalue (`GameplayStatics.GetPlayerController` 0))
  (set `self.IsActivated` true)
  (set `/Game/MyContent/BP/BP_Satellite.IsOnRail` true (`self.LinkedSatellite`))
  (`WidgetBlueprintLibrary.SetInputMode_GameOnly` _returnvalue)
  (set `PlayerController.bShowMouseCursor` false _returnvalue))

(fn `UserConstructionScript`)