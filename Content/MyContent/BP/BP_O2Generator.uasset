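; Oxygen generator Blueprint that can be damaged and repaired, mirroring its damaged state onto the first-person player character.
; DamageGenerator lowers HP and starts a red blink, while RepairGenerator restores HP and clears both at full health.
; Tick shows a repair bar widget driven by RepairProgress, separate from GeneratorHP, while damaged.
; Looping timers flip the tank material for red or green blinking, though nothing here triggers green.
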(event `self.ReceiveTick`
  (params (DeltaSeconds :type "Float (single-precision)"))
  (bind _repairbar (`self.RepairBar`))
  (if (`self.IsGeneratorDamaged`)
    (`SceneComponent.SetVisibility` _repairbar true false)
    (bind _asui_repair_bar (cast `/Game/MyContent/UI/UI_RepairBar` (`WidgetComponent.GetUserWidgetObject` _repairbar)))
    (`ProgressBar.SetPercent` (`/Game/MyContent/UI/UI_RepairBar.PB_Repair` _asui_repair_bar) (/ (`self.RepairProgress`) 100.0))
    (else
      (`SceneComponent.SetVisibility` (`self.RepairBar`) false false))))

(event `BlinkRed`
  (bind _oxygen_tank (`self.oxygen_tank`))
  (`/Engine/EditorBlueprintResources/StandardMacros.FlipFlop`
    (:`A`
      (`PrimitiveComponent.SetMaterial` _oxygen_tank 0 (`self.RedMaterial`)))
    (:`B`
      (`PrimitiveComponent.SetMaterial` _oxygen_tank 0 (`self.NormalMaterial`)))))

(event `StartBlinkRed`
  (bind _returnvalue (`KismetSystemLibrary.K2_SetTimer` null "BlinkRed" 0.3 true))
  (set `self.BlinkTimerHandle` _returnvalue)
  (set `self.IsBlinkingRed` true))

(event `StopBlink`
  (`KismetSystemLibrary.K2_ClearAndInvalidateTimerHandle` (`self.BlinkTimerHandle`))
  (set `self.IsBlinkingRed` false)
  (`PrimitiveComponent.SetMaterial` (`self.oxygen_tank`) 0 (`self.NormalMaterial`)))

(event `BlinkGreen`
  (bind _oxygen_tank (`self.oxygen_tank`))
  (`/Engine/EditorBlueprintResources/StandardMacros.FlipFlop`
    (:`A`
      (`PrimitiveComponent.SetMaterial` _oxygen_tank 0 (`self.GreenMaterial`)))
    (:`B`
      (`PrimitiveComponent.SetMaterial` _oxygen_tank 0 (`self.NormalMaterial`)))))

(event `StartBlinkGreen`
  (`self.StopBlink`)
  (bind _returnvalue (`KismetSystemLibrary.K2_SetTimer` null "BlinkGreen" 0.3 true))
  (set `self.BlinkTimerHandle` _returnvalue))

(fn `DamageGenerator`
  (set `self.IsGeneratorDamaged` true)
  (set `self.GeneratorHP` (`KismetMathLibrary.FClamp` (- (`self.GeneratorHP`) 8.0) 0.0 100.0))
  (bind _asbp_first_person_character (cast `/Game/FirstPerson/Blueprints/BP_FirstPersonCharacter` (`GameplayStatics.GetPlayerCharacter` 0)))
  (set `/Game/FirstPerson/Blueprints/BP_FirstPersonCharacter.IsO2GeneratorDamaged` true _asbp_first_person_character)
  (`self.StartBlinkRed`))

(fn `RepairGenerator`
  (bind _output_get (set `self.GeneratorHP` (`KismetMathLibrary.FClamp` (+ (`self.GeneratorHP`) (`self.RepairAmount`)) 0.0 100.0)))
  (if (>= _output_get 100.0)
    (set `self.IsGeneratorDamaged` false)
    (bind _asbp_first_person_character (cast `/Game/FirstPerson/Blueprints/BP_FirstPersonCharacter` (`GameplayStatics.GetPlayerCharacter` 0)))
    (set `/Game/FirstPerson/Blueprints/BP_FirstPersonCharacter.IsO2GeneratorDamaged` false _asbp_first_person_character)
    (`self.StopBlink`)))

(fn `UserConstructionScript`)